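; BP_Monster is an AI enemy that chases and hurts the player, with a camera-facing HP bar widget.
; Tick reads the blackboard's isSeePlayer to switch between faster and slower walk speed.
; A Box overlap sets isAttack and starts a looping timer that applies damage to the player, cleared on exit.
; AnyDamage lowers HP; at zero the mesh ragdolls, the player's kill count rises and the actor is destroyed after a delay.
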(event OnComponentBeginOverlap(Box)
  (params (OverlappedComponent :type Primitive%20Component%20Object%20Reference) (OtherActor :type Actor%20Object%20Reference) (OtherComp :type Primitive%20Component%20Object%20Reference) (OtherBodyIndex :type Integer) (bFromSweep :type Boolean) (SweepResult :type Hit%20Result%20Structure%20%28by%20ref%29))
  (bind _monster_blackboard (Variables|Default|GetMonster_Blackboard))
  (Utilities|IsValid _monster_blackboard
    (:Is%20Valid
      (AI|Components|Blackboard|SetValueasBool _monster_blackboard (Utilities|Name|MakeLiteralName "isAttack") true)
      (if (ScalableFloat|GetValueasBool (Variables|Default|GetMonster_Blackboard) (Utilities|Name|MakeLiteralName "isAttack"))
        (bind _returnvalue (Utilities|Time|SetTimerbyEvent (delegate Custom|Attack) 2.0 true))
        (else
          (Utilities|Time|ClearandInvalidateTimerbyHandle _returnvalue))))))

(event OnComponentEndOverlap(Box)
  (params (OverlappedComponent :type Primitive%20Component%20Object%20Reference) (OtherActor :type Actor%20Object%20Reference) (OtherComp :type Primitive%20Component%20Object%20Reference) (OtherBodyIndex :type Integer))
  (bind _monster_blackboard (Variables|Default|GetMonster_Blackboard))
  (Utilities|IsValid _monster_blackboard
    (:Is%20Valid
      (AI|Components|Blackboard|SetValueasBool _monster_blackboard (Utilities|Name|MakeLiteralName "isAttack") false)
      (if (ScalableFloat|GetValueasBool (Variables|Default|GetMonster_Blackboard) (Utilities|Name|MakeLiteralName "isAttack"))
        (bind _returnvalue (Utilities|Time|SetTimerbyEvent (delegate Custom|Attack) 2.0 true))
        (else
          (Utilities|Time|ClearandInvalidateTimerbyHandle _returnvalue))))))

(event Custom|Attack
  (bind _asbp_player (Utilities|Casting|CastToBP_Player (Game|Player|GetPlayerPawn 0)))
  (Game|Damage|ApplyDamage _asbp_player (Variables|Default|GetAttackValue) 0 0))

(event EventBeginPlay
  (Variables|Default|SetMonster_Blackboard (AI|GetBlackboard (AI|GetAIController self)))
  (bind _asbp_monster_hpbar (Utilities|Casting|CastToBP_MonsterHPBar (UserInterface|GetUserWidgetObject (Variables|Default|GetHPBar))))
  (Default|GetMonster _asbp_monster_hpbar self))

(event EventTick
  (params (DeltaSeconds :type Float%20%28single-precision%29))
  (bind _charactermovement (Variables|Character|GetCharacterMovement))
  (Utilities|FlowControl|Sequence
    (:then_0
      (Transformation|SetWorldRotation (Variables|Default|GetHPBar) (Math|Rotator|FindLookatRotation (Transformation|GetActorLocation) (Camera|GetCameraLocation (Game|GetPlayerCameraManager 0))) false false))
    (:then_1
      (if (ScalableFloat|GetValueasBool (Variables|Default|GetMonster_Blackboard) (Utilities|Name|MakeLiteralName "isSeePlayer")) ; True表示看到玩家，False表示丢失玩家
        (Variables|/Script/Engine.CharacterMovementComponent|SetMaxWalkSpeed _charactermovement 3e+02)
        (else
          (Variables|/Script/Engine.CharacterMovementComponent|SetMaxWalkSpeed _charactermovement 2e+02)))
      (if (<= (Variables|Default|GetHP) 0.0)
        (Utilities|FlowControl|DoOnce false
          (:Completed
            (Physics|SetSimulatePhysics (Variables|Character|GetMesh) true)
            (bind _asbp_player (Utilities|Casting|CastToBP_Player (Game|GetPlayerCharacter 0)))
            (Math|Integer|IncrementInt (Variables|/Game/Blueprints/Player/BP_Player.BP_Player_C|GetKilledNumber _asbp_player)
              (:%20%20
                (Utilities|FlowControl|Delay 3.0)
                (Actor|DestroyActor)))))))))

(event Game|Damage|EventAnyDamage
  (params (Damage :type Float%20%28single-precision%29) (DamageType :type Damage%20Type%20Object%20Reference) (InstigatedBy :type Controller%20Object%20Reference) (DamageCauser :type Actor%20Object%20Reference))
  (Variables|Default|SetHP (- (Variables|Default|GetHP) Damage)))

(fn ConstructionScript)
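; BP_JudgeBeenToAddres is a trigger actor that records when the player has reached an address and shows a destination widget.
; While BP_Player's IsOpenSwitch is false, Box overlap sets IsBeenToAddress and adds the BP_Destination widget, which end overlap removes.
; If IsOpenSwitch is true on overlap, the Box destroys itself through a DoOnce.
; Overlap events check player character 0 rather than the overlapping actor.
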(event OnComponentBeginOverlap(Box)
  (params (OverlappedComponent :type Primitive%20Component%20Object%20Reference) (OtherActor :type Actor%20Object%20Reference) (OtherComp :type Primitive%20Component%20Object%20Reference) (OtherBodyIndex :type Integer) (bFromSweep :type Boolean) (SweepResult :type Hit%20Result%20Structure%20%28by%20ref%29))
  (bind _asbp_player (Utilities|Casting|CastToBP_Player (Game|GetPlayerCharacter 0)))
  (if (Variables|/Game/Blueprints/Player/BP_Player.BP_Player_C|GetisOpenSwitch _asbp_player)
    (Utilities|FlowControl|DoOnce false
      (:Completed
        (Components|DestroyComponent (Variables|Default|GetBox))))
    (else
      (Variables|/Game/Blueprints/Player/BP_Player.BP_Player_C|SetisBeenToAddress _asbp_player true)
      (bind _returnvalue (UserInterface|CreateWidget "/Game/Blueprints/UI/ConmunicationUI/BP_Destination.BP_Destination_C" (Game|GetPlayerController 0)))
      (bind _output_get (Variables|Default|SetUI_Text _returnvalue))
      (UserInterface|Viewport|AddtoViewport _output_get 0))))

(event OnComponentEndOverlap(Box)
  (params (OverlappedComponent :type Primitive%20Component%20Object%20Reference) (OtherActor :type Actor%20Object%20Reference) (OtherComp :type Primitive%20Component%20Object%20Reference) (OtherBodyIndex :type Integer))
  (bind _asbp_player (Utilities|Casting|CastToBP_Player (Game|GetPlayerCharacter 0)))
  (if (not (Variables|/Game/Blueprints/Player/BP_Player.BP_Player_C|GetisOpenSwitch _asbp_player))
    (Widget|RemovefromParent (Variables|Default|GetUI_Text))))

(event EventBeginPlay)

(event Collision|EventActorBeginOverlap
  (params (OtherActor :type Actor%20Object%20Reference)))

(event EventTick
  (params (DeltaSeconds :type Float%20%28single-precision%29)))

(fn ConstructionScript)
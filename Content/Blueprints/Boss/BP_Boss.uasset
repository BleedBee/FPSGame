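; Boss enemy that fights the player and flags the player as the winner when it dies.
; Tick watches HP and Blackboard keys to show the boss HP bar when battle begins and handle death with a delayed destroy.
; The Attack overlap drives a looping timer of basic damage while the player stays inside.
; Skill damage lands once per isSkillAttack activation if the player is in the SkillAttack volume, using a resettable DoOnce.
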(event OnComponentBeginOverlap(Attack)
  (params (OverlappedComponent :type Primitive%20Component%20Object%20Reference) (OtherActor :type Actor%20Object%20Reference) (OtherComp :type Primitive%20Component%20Object%20Reference) (OtherBodyIndex :type Integer) (bFromSweep :type Boolean) (SweepResult :type Hit%20Result%20Structure%20%28by%20ref%29))
  (bind _blackboard (Variables|Default|GetBlackboard))
  (Utilities|IsValid _blackboard
    (:Is%20Valid
      (AI|Components|Blackboard|SetValueasBool _blackboard (Utilities|Name|MakeLiteralName "isAttack") true)
      (Utilities|FlowControl|RetriggerableDelay 0.5)
      (if (ScalableFloat|GetValueasBool (Variables|Default|GetBlackboard) (Utilities|Name|MakeLiteralName "isAttack"))
        (CallFunction|BossAttack)
        (bind _returnvalue (Utilities|Time|SetTimerbyEvent (delegate Custom|BossAttack) 3.0 true))
        (Variables|Default|SetBossAttackHandle _returnvalue)))))

(event OnComponentEndOverlap(Attack)
  (params (OverlappedComponent :type Primitive%20Component%20Object%20Reference) (OtherActor :type Actor%20Object%20Reference) (OtherComp :type Primitive%20Component%20Object%20Reference) (OtherBodyIndex :type Integer))
  (bind _blackboard (Variables|Default|GetBlackboard))
  (Utilities|IsValid _blackboard
    (:Is%20Valid
      (AI|Components|Blackboard|SetValueasBool _blackboard (Utilities|Name|MakeLiteralName "isAttack") false)
      (if (Utilities|Time|IsValidTimerHandle (Variables|Default|GetBossAttackHandle))
        (Utilities|Time|ClearandInvalidateTimerbyHandle (Variables|Default|GetBossAttackHandle))))))

(event OnComponentBeginOverlap(SkillAttack)
  (params (OverlappedComponent :type Primitive%20Component%20Object%20Reference) (OtherActor :type Actor%20Object%20Reference) (OtherComp :type Primitive%20Component%20Object%20Reference) (OtherBodyIndex :type Integer) (bFromSweep :type Boolean) (SweepResult :type Hit%20Result%20Structure%20%28by%20ref%29))
  (Variables|Default|SetisPlayerInSkillAttackRange true))

(event OnComponentEndOverlap(SkillAttack)
  (params (OverlappedComponent :type Primitive%20Component%20Object%20Reference) (OtherActor :type Actor%20Object%20Reference) (OtherComp :type Primitive%20Component%20Object%20Reference) (OtherBodyIndex :type Integer))
  (Variables|Default|SetisPlayerInSkillAttackRange false))

(event Custom|BossAttack
  (bind _asbp_player (Utilities|Casting|CastToBP_Player (Game|Player|GetPlayerPawn 0)))
  (Game|Damage|ApplyDamage _asbp_player (Variables|Default|GetBossAttackValue) 0 0))

(event EventBeginPlay
  (Utilities|FlowControl|Delay 0.5)
  (Variables|Default|SetBlackboard (AI|GetBlackboard (AI|GetAIController self))))

(event EventTick
  (params (DeltaSeconds :type Float%20%28single-precision%29))
  (Utilities|FlowControl|Sequence
    (:then_0
      (if (<= (Variables|Default|GetHP) 0.0)
        (Utilities|FlowControl|DoOnce false
          (:Completed
            (AI|Navigation|StopMovement (AI|GetAIController self))
            (AI|Components|Blackboard|SetValueasBool (Variables|Default|GetBlackboard) (Utilities|Name|MakeLiteralName "isDeath") true)
            (Widget|RemovefromParent (Variables|Default|GetHPBar))
            (Utilities|FlowControl|Delay 3.5)
            (bind _asbp_player (Utilities|Casting|CastToBP_Player (Game|GetPlayerCharacter 0)))
            (Variables|/Game/Blueprints/Player/BP_Player.BP_Player_C|SetisWin _asbp_player true)
            (Actor|DestroyActor)))))
    (:then_1
      (if (ScalableFloat|GetValueasBool (Variables|Default|GetBlackboard) (Utilities|Name|MakeLiteralName "isBeginBossBattle"))
        (Utilities|FlowControl|DoOnce false
          (:Completed
            (bind _returnvalue (UserInterface|CreateWidget "/Game/Blueprints/UI/BossUI/BP_BossHPBar.BP_BossHPBar_C"))
            (Variables|Default|SetHPBar _returnvalue)
            (UserInterface|Viewport|AddtoViewport (Variables|Default|GetHPBar) 0)))))
    (:then_2
      (if (and (Variables|Default|GetisPlayerInSkillAttackRange) (ScalableFloat|GetValueasBool (Variables|Default|GetBlackboard) (Utilities|Name|MakeLiteralName "isSkillAttack")))
        (Utilities|FlowControl|DoOnce false :!label _label
          (:Completed
            (bind _asbp_player_2 (Utilities|Casting|CastToBP_Player (Game|Player|GetPlayerPawn 0)))
            (Game|Damage|ApplyDamage _asbp_player_2 (Variables|Default|GetBossSkillAttackValue) 0 0)))))
    (:then_3
      (if (not (ScalableFloat|GetValueasBool (Variables|Default|GetBlackboard) (Utilities|Name|MakeLiteralName "isSkillAttack")))
        (goto _label Reset)))))

(event Game|Damage|EventAnyDamage
  (params (Damage :type Float%20%28single-precision%29) (DamageType :type Damage%20Type%20Object%20Reference) (InstigatedBy :type Controller%20Object%20Reference) (DamageCauser :type Actor%20Object%20Reference))
  (Variables|Default|SetHP (- (Variables|Default|GetHP) Damage)))

(fn ConstructionScript)
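; BP_FallDeath is an interactive actor whose Box trigger ends the game, apparently as a fall-death zone.
; BeginPlay caches the player character as BP_Player.
; Any overlap with the Box, with no check on the overlapping actor, removes the player's UI and shows a BP_GameOver widget.
; It then switches input to UI only, shows the mouse cursor and pauses the game.
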(event OnComponentBeginOverlap(Box)
  (params (OverlappedComponent :type Primitive%20Component%20Object%20Reference) (OtherActor :type Actor%20Object%20Reference) (OtherComp :type Primitive%20Component%20Object%20Reference) (OtherBodyIndex :type Integer) (bFromSweep :type Boolean) (SweepResult :type Hit%20Result%20Structure%20%28by%20ref%29))
  (bind _returnvalue (Game|GetPlayerController 0))
  (Widget|RemovefromParent (Variables|/Game/Blueprints/Player/BP_Player.BP_Player_C|GetPlayerUI (Variables|Default|GetBP_Player)))
  (bind _returnvalue_2 (UserInterface|CreateWidget "/Game/Blueprints/UI/GameFramework/BP_GameOver.BP_GameOver_C" (Game|GetPlayerController 0)))
  (UserInterface|Viewport|AddtoViewport _returnvalue_2 0)
  (Input|SetInputModeUIOnly _returnvalue 0 "DoNotLock")
  (Variables|/Script/Engine.PlayerController|SetbShowMouseCursor _returnvalue true)
  (Game|SetGamePaused true))

(event EventBeginPlay
  (bind _asbp_player (Utilities|Casting|CastToBP_Player (Game|GetPlayerCharacter 0)))
  (Variables|Default|SetBP_Player _asbp_player))

(event Collision|EventActorBeginOverlap
  (params (OtherActor :type Actor%20Object%20Reference)))

(event EventTick
  (params (DeltaSeconds :type Float%20%28single-precision%29)))

(fn ConstructionScript)
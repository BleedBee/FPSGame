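; Interactive switch that the player triggers with F inside its box to lower the actor tagged WinPoint.
; Box overlap enables input and shows BP_InteractiveTip if BP_Player's IsBeenToAddress is set, otherwise BP_SwitchUI; leaving reverses both.
; F works once, only with that flag set: it sets IsOpenSwitch, removes the tip and runs the WinPointDown timeline on the target's Z, then destroys the box.
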(event OnComponentBeginOverlap(Box)
  (params (OverlappedComponent :type Primitive%20Component%20Object%20Reference) (OtherActor :type Actor%20Object%20Reference) (OtherComp :type Primitive%20Component%20Object%20Reference) (OtherBodyIndex :type Integer) (bFromSweep :type Boolean) (SweepResult :type Hit%20Result%20Structure%20%28by%20ref%29))
  (bind _asbp_player (Utilities|Casting|CastToBP_Player (Game|GetPlayerCharacter 0)))
  (if (Variables|/Game/Blueprints/Player/BP_Player.BP_Player_C|GetisOpenSwitch _asbp_player)
    (Utilities|FlowControl|DoOnce false
      (:Completed
        (Components|DestroyComponent (Variables|Default|GetBox))))
    (else
      (Input|EnableInput (Game|GetPlayerController 0))
      (bind _asbp_player_2 (Utilities|Casting|CastToBP_Player (Game|GetPlayerCharacter 0)))
      (if (Variables|/Game/Blueprints/Player/BP_Player.BP_Player_C|GetisBeenToAddress _asbp_player_2)
        (bind _returnvalue (UserInterface|CreateWidget "/Game/Blueprints/UI/ConmunicationUI/BP_InteractiveTip.BP_InteractiveTip_C" (Game|GetPlayerController 0)))
        (bind _output_get (Variables|Default|SetUI_TipText _returnvalue))
        (UserInterface|Viewport|AddtoViewport _output_get 0)
        (else
          (bind _returnvalue_2 (UserInterface|CreateWidget "/Game/Blueprints/UI/ConmunicationUI/BP_SwitchUI.BP_SwitchUI_C" (Game|GetPlayerController 0)))
          (bind _output_get_2 (Variables|Default|SetUI_Text _returnvalue_2))
          (UserInterface|Viewport|AddtoViewport _output_get_2 0))))))

(event OnComponentEndOverlap(Box)
  (params (OverlappedComponent :type Primitive%20Component%20Object%20Reference) (OtherActor :type Actor%20Object%20Reference) (OtherComp :type Primitive%20Component%20Object%20Reference) (OtherBodyIndex :type Integer))
  (bind _asbp_player (Utilities|Casting|CastToBP_Player (Game|GetPlayerCharacter 0)))
  (if (not (Variables|/Game/Blueprints/Player/BP_Player.BP_Player_C|GetisOpenSwitch _asbp_player))
    (Input|DisableInput (Game|GetPlayerController 0))
    (bind _asbp_player_2 (Utilities|Casting|CastToBP_Player (Game|GetPlayerCharacter 0)))
    (if (Variables|/Game/Blueprints/Player/BP_Player.BP_Player_C|GetisBeenToAddress _asbp_player_2)
      (Widget|RemovefromParent (Variables|Default|GetUI_TipText))
      (else
        (Widget|RemovefromParent (Variables|Default|GetUI_Text))))))

(event EventBeginPlay)

(event Collision|EventActorBeginOverlap
  (params (OtherActor :type Actor%20Object%20Reference)))

(event EventTick
  (params (DeltaSeconds :type Float%20%28single-precision%29)))

(event Input|KeyboardEvents|F
  (params (Key :type Key%20Structure))
  (:Pressed
    (bind _asbp_player (Utilities|Casting|CastToBP_Player (Game|GetPlayerCharacter 0)))
    (if (and (Variables|/Game/Blueprints/Player/BP_Player.BP_Player_C|GetisBeenToAddress _asbp_player) (not (Variables|/Game/Blueprints/Player/BP_Player.BP_Player_C|GetisOpenSwitch _asbp_player)))
      (Utilities|FlowControl|DoOnce false
        (:Completed
          (bind _asbp_player_2 (Utilities|Casting|CastToBP_Player (Game|GetPlayerCharacter 0)))
          (Variables|/Game/Blueprints/Player/BP_Player.BP_Player_C|SetisOpenSwitch _asbp_player_2 true)
          (Widget|RemovefromParent (Variables|Default|GetUI_TipText))
          (bind _outactors (Actor|GetAllActorswithTag "WinPoint"))
          (Variables|Default|SetWinPointZ (.z (Transformation|GetActorLocation (Utilities|Array|Get(acopy) _outactors))))
          (bind _alpha (Timeline|WinPointDown Play)
            (:Update
              (Transformation|SetActorLocation (Utilities|Array|Get(acopy) _outactors) (Math|Vector|MakeVector (.x (Transformation|GetActorLocation (Utilities|Array|Get(acopy) _outactors))) (.y (Transformation|GetActorLocation (Utilities|Array|Get(acopy) _outactors))) (- (Variables|Default|GetWinPointZ) _alpha)) false false))
            (:Finished
              (Components|DestroyComponent (Variables|Default|GetBox)))))))))

(fn ConstructionScript)
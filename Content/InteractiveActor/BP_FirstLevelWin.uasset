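; BP_FirstLevelWin is a trigger actor that ends the first level and moves the game on to BossLevel.
; When anything overlaps its Box, it copies player character 0's HP and both bullet counts into BP_GameInstance so they outlive the level change.
; After a short delay it sets OpenLevelMode on the game instance and opens the boss map by name.
; The overlapping actor itself is never checked.
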(event OnComponentBeginOverlap(Box)
  (params (OverlappedComponent :type Primitive%20Component%20Object%20Reference) (OtherActor :type Actor%20Object%20Reference) (OtherComp :type Primitive%20Component%20Object%20Reference) (OtherBodyIndex :type Integer) (bFromSweep :type Boolean) (SweepResult :type Hit%20Result%20Structure%20%28by%20ref%29))
  (bind _asbp_player (Utilities|Casting|CastToBP_Player (Game|GetPlayerCharacter 0)))
  (bind _asbp_game_instance (Utilities|Casting|CastToBP_GameInstance (Game|GetGameInstance)))
  (Variables|/Game/Blueprints/BP_GameInstance.BP_GameInstance_C|SetPlayerHP _asbp_game_instance (Variables|/Game/Blueprints/Player/BP_Player.BP_Player_C|GetHP _asbp_player))
  (Variables|/Game/Blueprints/BP_GameInstance.BP_GameInstance_C|SetPlayerCurrentBulletNum _asbp_game_instance (Variables|/Game/Blueprints/Player/BP_Player.BP_Player_C|GetCurrentBulletNum _asbp_player))
  (Variables|/Game/Blueprints/BP_GameInstance.BP_GameInstance_C|SetPlayerPrepareBulletNum _asbp_game_instance (Variables|/Game/Blueprints/Player/BP_Player.BP_Player_C|GetPrepareBulletNum _asbp_player))
  (Utilities|FlowControl|Delay 1.0)
  (Variables|/Game/Blueprints/BP_GameInstance.BP_GameInstance_C|SetOpenLevelMode _asbp_game_instance 1)
  (Game|OpenLevel(byName) "BossLevel"))

(event EventBeginPlay)

(event Collision|EventActorBeginOverlap
  (params (OtherActor :type Actor%20Object%20Reference)))

(event EventTick
  (params (DeltaSeconds :type Float%20%28single-precision%29)))

(fn ConstructionScript)